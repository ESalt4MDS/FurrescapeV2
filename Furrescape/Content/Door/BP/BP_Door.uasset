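; BP_Door is a door that slides straight up when unlocked.
; On BeginPlay it caches the mesh's relative location as closed and derives the open position from a fixed Z offset.
; The UnlockOpen event clears the lock and, if the door is not yet open, plays a timeline that lerps the mesh between those positions.
; When the timeline finishes it marks the door open and prints a message; no closing logic exists.
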(event Custom|UnlockOpen
  ;[0.15 0.15 0.15 0.5] DoorOpen when it is unlocked
  (Variables|Default|SetIsLocked false)
  (if (not (Variables|Default|GetIsOpen))
    (bind _alpha (Timeline|OpenTimeline PlayFromStart)
      (:Update
        (Transformation|SetRelativeLocation (Variables|Default|GetDoorMesh) (Math|Vector|Lerp(Vector) (Variables|Default|GetClosedLocation) (Variables|Default|GetOpenLocation) _alpha) false false))
      (:Finished
        (Variables|Default|SetIsOpen true)
        (Development|PrintString "It Opened")))))

(event EventBeginPlay
  ;[0.15 0.15 0.15 0.5] Closed Door
  (Variables|Default|SetClosedLocation (Variables|/Script/Engine.SceneComponent|GetRelativeLocation (Variables|Default|GetDoorMesh)))
  ;[0.15 0.15 0.15 0.5] Door is Open
  (Variables|Default|SetOpenLocation (+ (Variables|Default|GetClosedLocation) "0.000000,0.000000,800.000000")))

(event Collision|EventActorBeginOverlap
  (params (OtherActor :type Actor%20Object%20Reference)))

(event EventTick
  (params (DeltaSeconds :type Float%20%28single-precision%29)))

(fn ConstructionScript)