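; AI controller for an NPC that runs BT_NPCTree and feeds its blackboard from sight, hearing and prediction perception.
; Sight updates handle the player's target and last seen location, and request a predicted player position.
; Hearing and prediction handlers write TargetLocation, though the prediction branch compares against the sense config class instead of the sense class.
; The LastHeardLocation write is unreachable, and a GiveUp counter is left unconnected.
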(event OnTargetPerceptionUpdated(AIPerception)
  (params (Actor :type Actor%20Object%20Reference) (Stimulus :type AI%20Stimulus%20Structure))
  (bind _returnvalue (Class|AIPerceptionSystem|GetSenseClassforStimulus Stimulus))
  (Utilities|FlowControl|Sequence
    (:then_0
      (if (== _returnvalue "/Script/AIModule.AISense_Sight")
        (CallFunction|HandleSight Actor Stimulus)))
    (:then_1
      (if (== _returnvalue "/Script/AIModule.AISense_Hearing")
        (CallFunction|HandleHearing Stimulus)))
    (:then_2
      (if (== _returnvalue "/Script/AIModule.AISenseConfig_Prediction")
        (CallFunction|HandlePrediction Stimulus)))))

(event EventBeginPlay
  (AI|RunBehaviorTree "/Game/NPC/BT_NPCTree.BT_NPCTree")
  (AI|Components|Blackboard|SetValueasObject (AI|GetBlackboard 0) (Utilities|Name|MakeLiteralName "SelfActor") "/Game/NPC/BP_NPC.BP_NPC"))

(fn ConstructionScript)

(fn HandleSight
  (params (Actor :type Actor%20Object%20Reference) (Stimulus :type AI%20Stimulus%20Structure))
  (bind (_age _expirationage _strength _stimuluslocation _receiverlocation _tag _bsuccessfullysensed) (Utilities|Struct|BreakAIStimulus Stimulus))
  (bind _returnvalue (Game|GetPlayerCharacter 0))
  (bind _returnvalue_2 (== Actor _returnvalue))
  (AI|Components|Blackboard|SetValueasBool (AI|GetBlackboard 0) (Utilities|Name|MakeLiteralName "IsPlayerInsight") _returnvalue_2)
  (if _returnvalue_2
    (Class|AISensePrediction|RequestPawnPredictionEvent (Pawn|GetControlledPawn) (Game|GetPlayerCharacter 0) 1.5)
    (AI|Components|Blackboard|SetValueasObject (AI|GetBlackboard 0) (Utilities|Name|MakeLiteralName "TargetActor") (Utilities|SelectObject Actor 0 _bsuccessfullysensed))
    (if (not _bsuccessfullysensed)
      ;[0.15 0.15 0.15 0.5] if NPC can Not see the tartgetActor Save last seen location
      (AI|Components|Blackboard|SetValueasVector (AI|GetBlackboard 0) (Utilities|Name|MakeLiteralName "LastSeenLocation") _stimuluslocation))
    (else
      (return))))

(fn HandleHearing
  (params (Stimulus :type AI%20Stimulus%20Structure))
  (if (.bsuccessfullysensed Stimulus)
    (AI|Components|Blackboard|SetValueasVector (AI|GetBlackboard 0) (Utilities|Name|MakeLiteralName "TargetLocation") (.stimuluslocation Stimulus))
    ;[0.15 0.15 0.15 0.5] if NPC can Not see the tartgetActor Save last seen location
    (if (not (.bsuccessfullysensed Stimulus))
      (AI|Components|Blackboard|SetValueasVector (AI|GetBlackboard 0) (Utilities|Name|MakeLiteralName "LastHeardLocation") (.stimuluslocation Stimulus)))
    (else
      (return))))

(fn HandlePrediction
  (params (Stimulus :type AI%20Stimulus%20Structure))
  (bind (_age _expirationage _strength _stimuluslocation _receiverlocation _tag _bsuccessfullysensed) (Utilities|Struct|BreakAIStimulus Stimulus))
  (if _bsuccessfullysensed
    (AI|Components|Blackboard|SetValueasVector (AI|GetBlackboard 0) (Utilities|Name|MakeLiteralName "TargetLocation") _stimuluslocation)
    (else
      (return))))